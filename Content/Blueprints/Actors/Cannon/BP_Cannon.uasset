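; A cannon actor that automatically fires projectiles in a repeating loop from BeginPlay.
; After a configurable delay it spawns a BP_Projectile at the spawn point's location and rotation, using a configurable scale.
; A timeline animates barrel recoil along its local Y axis, and its Cannon Fired event track loops back to the delay for the next shot.
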(event `self.ReceiveBeginPlay`
  (`KismetSystemLibrary.Delay` (`self.DelayAmount`) :!label _label)
  (`self.Spawn Projectile`)
  (bind (_direction _cannon_barrel_recoil) (`Timeline|Cannon Fire Timeline` :!via `PlayFromStart`)
    (:`Update`
      (`self.MoveCannonBarrel` _cannon_barrel_recoil))
    (:`Cannon Fired`
      (goto _label))))

(fn `MoveCannonBarrel`
  (params (CannonBarrelYLocation :type "Float (double-precision)"))
  (`SceneComponent.K2_SetRelativeLocation` (`self.CannonBarrel`) (`KismetMathLibrary.MakeVector` 0.0 CannonBarrelYLocation) false false))

(fn `Spawn Projectile`
  (bind _projectilespawnpoint (`self.ProjectileSpawnPoint`))
  (`|SpawnActorFromClass` "/Game/Blueprints/Actors/Projectiles/BP_Projectile.BP_Projectile_C" (`KismetMathLibrary.MakeTransform` (`SceneComponent.K2_GetComponentLocation` _projectilespawnpoint) (`SceneComponent.K2_GetComponentRotation` _projectilespawnpoint) (`KismetMathLibrary.Conv_DoubleToVector` (`self.ProjectileScale`))) "Undefined" "OverrideRootScale" null null))

(fn `UserConstructionScript`)